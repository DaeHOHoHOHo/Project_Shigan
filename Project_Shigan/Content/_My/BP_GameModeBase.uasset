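; Game mode that persists the start menu controller's SkillGold in a single save slot through BP_SaveGame.
; BeginPlay copies saved gold into Controller_StartMenu, or creates an empty save if none exists.
; SaveGame writes the controller's current gold back to the slot.
; LoadGame restarts the level so BeginPlay re-reads the save, while RestartLevel deletes the save before restarting.
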(event Custom|SaveGame
  (bind _returnvalue (SaveGame|LoadGamefromSlot "save1"))
  (bind _asbp_save_game (Utilities|Casting|CastToBP_SaveGame _returnvalue))
  (Variables|/Game/_My/BP_SaveGame.BP_SaveGame_C|SetSaveGold _asbp_save_game (Variables|/Script/Project_Shigan.Controller_StartMenu|GetskillGold (.AsController%20Start%20Menu (Utilities|Casting|CastToController_StartMenu (Game|GetPlayerController 0)))))
  (SaveGame|SaveGametoSlot _asbp_save_game "save1"))

(event Custom|LoadGame
  (Development|ExecuteConsoleCommand "RestartLevel" 0))

(event Custom|RestartLevel
  (SaveGame|DeleteGameinSlot "save1")
  (Development|ExecuteConsoleCommand "RestartLevel" 0))

(event EventBeginPlay
  (SaveGame|DoesSaveGameExist "save1")
  (if true
    (bind _returnvalue (SaveGame|LoadGamefromSlot "save1"))
    (bind _asbp_save_game (Utilities|Casting|CastToBP_SaveGame _returnvalue))
    (bind _ascontroller_start_menu (Utilities|Casting|CastToController_StartMenu (Game|GetPlayerController 0)))
    (Variables|/Script/Project_Shigan.Controller_StartMenu|SetskillGold _ascontroller_start_menu (Variables|/Game/_My/BP_SaveGame.BP_SaveGame_C|GetSaveGold _asbp_save_game))
    (else
      (bind _returnvalue_2 (SaveGame|CreateSaveGameObject "/Game/_My/BP_SaveGame.BP_SaveGame_C"))
      (SaveGame|SaveGametoSlot _returnvalue_2 "save1"))))

(fn ConstructionScript)