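; Player character Blueprint handling melee combat, weapon and item pickup, camera switching, and HUD, inventory and skill tree UI.
; Input plays montages to pick up, draw and sheathe weapons.
; One- and two-handed sword combos buffer clicks during attacks, advanced through combo events.
; Damage while blocking notifies the attacker if facing yaws roughly oppose; otherwise it sets health, plays a hit reaction and clears attack state.
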(event Custom|DrawWeapon
  ;[1 1 1] Draw/Sheathe Weapon
  (Transformation|AttachComponentToComponent (Variables|Default|GetEquippedWeapon) (Variables|Character|GetMesh) "RightHandWeapon" "SnapToTarget" "SnapToTarget" "SnapToTarget" true)
  (Variables|Default|SetWeaponDrawn true))

(event Custom|SheatheWeapon
  ;[1 1 1] Draw/Sheathe Weapon
  (Transformation|AttachComponentToComponent (Variables|Default|GetEquippedWeapon) (Variables|Character|GetMesh) "Weapon_Back" "SnapToTarget" "SnapToTarget" "SnapToTarget" true)
  (Variables|Default|SetWeaponDrawn false))

(event Custom|OpenST
  (Default|Open/CloseST (Variables|Default|GetST) true)
  (Input|SetInputModeGameandUI (Game|GetPlayerController 0) (Variables|Default|GetST) "LockOnCapture" false)
  (Variables|/Script/Engine.PlayerController|SetbShowMouseCursor (Game|GetPlayerController 0) true)
  (Variables|Default|SetisSTVisible true))

(event Custom|CloseST
  (Default|Open/CloseST (Variables|Default|GetST) false)
  (Input|SetInputModeGameOnly (Game|GetPlayerController 0))
  (Variables|/Script/Engine.PlayerController|SetbShowMouseCursor (Game|GetPlayerController 0) false)
  (Variables|Default|SetisSTVisible false))

(event Custom|OneHandSwordCombo
  ;[1 1 1] One Hand Sword
  (if (Variables|OneHand|GetSaveAttack_OneHand)
    (Variables|OneHand|SetSaveAttack_OneHand false)
    (switch int (Variables|OneHand|GetAttackCounter_OneHand)
      (:0
        (Variables|OneHand|SetAttackCounter_OneHand 1)
        (Animation|PlayAnimMontage "/Game/_My/Weapon/Attack_Anim/OneHandSword_Attack1.OneHandSword_Attack1" 1.0 "None"))
      (:1
        (Variables|OneHand|SetAttackCounter_OneHand 2)
        (Animation|PlayAnimMontage "/Game/_My/Weapon/Attack_Anim/OneHandSword_Attack2.OneHandSword_Attack2" 1.0 "None"))
      (:2
        (Variables|OneHand|SetAttackCounter_OneHand 3)
        (Animation|PlayAnimMontage "/Game/_My/Weapon/Attack_Anim/OneHandSword_Attack3.OneHandSword_Attack3" 1.0 "None"))
      (:3
        (Variables|OneHand|SetAttackCounter_OneHand 0)
        (Animation|PlayAnimMontage "/Game/_My/Weapon/Attack_Anim/OneHandSword_Attack4.OneHandSword_Attack4" 1.0 "None")))
    (else
      (Variables|OneHand|SetAttackCounter_OneHand 0)
      (Variables|Default|SetAttacking false))))

(event Custom|TwoHandSwordCombo
  ;[1 1 1] Two Hand Sword
  (if (Variables|TwoHand|GetSaveAttack_TwoHand)
    (Variables|TwoHand|SetSaveAttack_TwoHand false)
    (switch int (Variables|TwoHand|GetAttackCounter_TwoHand)
      (:0
        (Variables|TwoHand|SetAttackCounter_TwoHand 1)
        (Animation|PlayAnimMontage "/Game/_My/Weapon/Attack_Anim/TwoHandSword_Attack1.TwoHandSword_Attack1" 1.0 "None"))
      (:1
        (Variables|TwoHand|SetAttackCounter_TwoHand 2)
        (Animation|PlayAnimMontage "/Game/_My/Weapon/Attack_Anim/TwoHandSword_Attack2.TwoHandSword_Attack2" 1.0 "None"))
      (:2
        (Variables|TwoHand|SetAttackCounter_TwoHand 0)
        (Animation|PlayAnimMontage "/Game/_My/Weapon/Attack_Anim/TwoHandSword_Attack3.TwoHandSword_Attack3" 1.0 "None")))
    (else
      (Variables|TwoHand|SetAttackCounter_TwoHand 0)
      (Variables|Default|SetAttacking false))))

(event EventDropAction
  (params (Item%20To%20Drop :type Actor%20Object%20Reference))
  ;[1 1 1] Drop Item
  (Rendering|SetActorHiddenInGame Item%20To%20Drop false)
  (Collision|SetActorEnableCollision Item%20To%20Drop true)
  (Transformation|SetActorTransform Item%20To%20Drop (Transformation|GetWorldTransform (Variables|Default|GetDropLocation))))

(event Game|Damage|EventAnyDamage
  (params (Damage :type Float%20%28single-precision%29) (DamageType :type Damage%20Type%20Object%20Reference) (InstigatedBy :type Controller%20Object%20Reference) (DamageCauser :type Actor%20Object%20Reference))
  ;[1 1 1] Damage
  (Variables|Default|SetDamage%20Causer DamageCauser)
  (if (Variables|Default|GetBlocking)
    (bind _facingai_ (CallFunction|BlockAngleCheck))
    (if _facingai_
      (Class|BPBlock|AttackBlocked(Message) DamageCauser)
      (Development|PrintString "Hello")
      (else
        (Variables|Default|SetHealth (- (Variables|Default|GetmyHPnum) Damage) :!label _label)
        (Animation|PlayAnimMontage "/Game/_My/Player/Player_BeHit_AnimMontage.Player_BeHit_AnimMontage" 1.0 "None")
        (Variables|OneHand|SetSaveAttack_OneHand false)
        (Variables|TwoHand|SetSaveAttack_TwoHand false)
        (Variables|Default|SetAttacking false)))
    (else
      (goto _label))))

(event EventBeginPlay
  ;[1 1 1] Event BeginPlay
  (Utilities|FlowControl|Sequence
    (:then_0
      (bind _returnvalue (UserInterface|CreateWidget "/Game/_My/UI/BP_HUD.BP_HUD_C"))
      (bind _output_get (Variables|Default|SetGameHUDReference _returnvalue))
      (UserInterface|Viewport|AddtoViewport _output_get 0)
      (CallFunction|DisalbeMouseCursor))
    (:then_1
      (bind _returnvalue_2 (UserInterface|CreateWidget "/Game/_My/UI/BP_SkillTree.BP_SkillTree_C"))
      (Variables|Default|SetST _returnvalue_2)
      (UserInterface|Viewport|AddtoViewport _returnvalue_2 0)
      (CallFunction|CloseST))))

(event Input|ActionEvents|InputActionSwitchCamera
  (params (Key :type Key%20Structure :default "None"))
  ;[1 1 1] change First/Third
  (:Pressed
    (Utilities|FlowControl|FlipFlop
      (:A
        (Components|Activation|SetActive (Variables|Default|GetFPSCamera) true false)
        (Components|Activation|SetActive (Variables|Default|GetFollowCamera) false false)
        (Variables|Default|SetbUseControllerRotationYaw true))
      (:B
        (Components|Activation|SetActive (Variables|Default|GetFPSCamera) false false)
        (Components|Activation|SetActive (Variables|Default|GetFollowCamera) true false)
        (Variables|Default|SetbUseControllerRotationYaw false)))))

(event Input|ActionEvents|InputActionOpen/CloseST
  (params (Key :type Key%20Structure :default "None"))
  (:Pressed
    (if (Variables|Default|GetisSTVisible)
      (CallFunction|CloseST)
      (else
        (CallFunction|OpenST)))))

(event Input|KeyboardEvents|I
  (params (Key :type Key%20Structure :default "None"))
  (bind _gamehudreference (Variables|Default|GetGameHUDReference))
  ;[1 1 1] Toggle Inventory Menu
  (:Pressed
    (if (Variables|/Game/_My/UI/BP_HUD.BP_HUD_C|GetActivateInventory _gamehudreference)
      (Utilities|FlowControl|FlipFlop
        (:A
          (Variables|/Game/_My/UI/BP_HUD.BP_HUD_C|SetInventoryVisible _gamehudreference "Visible")
          (CallFunction|EnableMouseCursor))
        (:B
          (Variables|/Game/_My/UI/BP_HUD.BP_HUD_C|SetInventoryVisible _gamehudreference "Hidden")
          (CallFunction|DisalbeMouseCursor))))))

(event Input|KeyboardEvents|E
  (params (Key :type Key%20Structure :default "None"))
  ;[1 1 1] Pickup Item
  (:Pressed
    (if (< (Utilities|Array|Length (Variables|/Game/_My/UI/BP_HUD.BP_HUD_C|GetInventory (Variables|Default|GetGameHUDReference))) 15)
      (Default|CallPickupItem))))

(event Input|MouseEvents|LeftMouseButton
  (params (Key :type Key%20Structure :default "None"))
  ;[1 1 1] EquipWeapon
  (:Pressed
    (if (not (Variables|Default|GetWeaponDrawn))
      (Utilities|IsValid (Variables|Default|GetEquippedWeapon)
        (:Is%20Valid
          (Utilities|FlowControl|DoOnce false :!label _label
            (:Completed
              (bind _returnvalue (Animation|PlayAnimMontage "/Game/_My/Player/Draw_Weapon_AnimMontage.Draw_Weapon_AnimMontage" 1.0 "None"))
              (Utilities|FlowControl|Delay _returnvalue)
              (Variables|Default|SetReadyToAttack true)
              (goto _label Reset))))))))

(event Input|MouseEvents|RightMouseButton
  (params (Key :type Key%20Structure :default "None"))
  (:Pressed
    (if (not (Variables|Default|GetisSTVisible))
      (Variables|Default|SetBlocking true)))
  (:Released
    (Variables|Default|SetBlocking false)))

(event Input|KeyboardEvents|Tab
  (params (Key :type Key%20Structure :default "None"))
  ;[1 1 1] UnEquipWeapon
  (:Pressed
    (if (not (Variables|Default|GetAttacking))
      (if (Variables|Default|GetWeaponDrawn)
        (Utilities|IsValid (Variables|Default|GetEquippedWeapon)
          (:Is%20Valid
            (Utilities|FlowControl|DoOnce false :!label _label
              (:Completed
                (bind _returnvalue (Animation|PlayAnimMontage "/Game/_My/Player/Sheathe_Weapon_AnimMontage.Sheathe_Weapon_AnimMontage" 1.0 "None"))
                (Utilities|FlowControl|Delay _returnvalue)
                (Variables|Default|SetReadyToAttack false)
                (goto _label Reset)))))))))

(event Input|KeyboardEvents|E
  (params (Key :type Key%20Structure :default "None"))
  ;[1 1 1] Get Weapon
  (:Pressed
    (bind _array_element (Utilities|Array|ForEachLoopwithBreak (Collision|GetOverlappingActors "/Script/Engine.Actor" :!class /Script/Engine.Actor) :!label _label)
      (:LoopBody
        (if (Utilities|DoesObjectImplementInterface _array_element "/Game/_My/Weapon/WeaponInterface.WeaponInterface_C")
          (if (!= _array_element (Variables|Default|GetEquippedWeapon))
            (if (not (Variables|Default|GetWeaponDrawn))
              (bind _returnvalue (Animation|PlayAnimMontage "/Game/_My/Player/PickUP_AnimMontage.PickUP_AnimMontage" 1.0 "None"))
              (Utilities|FlowControl|Delay _returnvalue)
              (Class|WeaponInterface|PickUpWeapon(Message) _array_element)
              (goto _label Break))))))))

(event Input|MouseEvents|LeftMouseButton
  (params (Key :type Key%20Structure :default "None"))
  (:Pressed
    (switch int (Variables|Default|GetWeaponType)
      (:1
        ;[1 1 1] One Hand Sword
        (if (Variables|Default|GetReadyToAttack)
          (if (Variables|Default|GetAttacking)
            (Variables|OneHand|SetSaveAttack_OneHand true)
            (else
              (Variables|Default|SetAttacking true)
              (switch int (Variables|OneHand|GetAttackCounter_OneHand)
                (:0
                  (Variables|OneHand|SetAttackCounter_OneHand 1)
                  (Animation|PlayAnimMontage "/Game/_My/Weapon/Attack_Anim/OneHandSword_Attack1.OneHandSword_Attack1" 1.0 "None"))
                (:1
                  (Variables|OneHand|SetAttackCounter_OneHand 2)
                  (Animation|PlayAnimMontage "/Game/_My/Weapon/Attack_Anim/OneHandSword_Attack2.OneHandSword_Attack2" 1.0 "None"))
                (:2
                  (Variables|OneHand|SetAttackCounter_OneHand 3)
                  (Animation|PlayAnimMontage "/Game/_My/Weapon/Attack_Anim/OneHandSword_Attack3.OneHandSword_Attack3" 1.0 "None"))
                (:3
                  (Variables|OneHand|SetAttackCounter_OneHand 0)
                  (Animation|PlayAnimMontage "/Game/_My/Weapon/Attack_Anim/OneHandSword_Attack4.OneHandSword_Attack4" 1.0 "None")))))))
      (:2
        ;[1 1 1] Two Hand Sword
        (if (Variables|Default|GetReadyToAttack)
          (if (Variables|Default|GetAttacking)
            (Variables|TwoHand|SetSaveAttack_TwoHand true)
            (else
              (Variables|Default|SetAttacking true)
              (switch int (Variables|TwoHand|GetAttackCounter_TwoHand)
                (:0
                  (Variables|TwoHand|SetAttackCounter_TwoHand 1)
                  (Animation|PlayAnimMontage "/Game/_My/Weapon/Attack_Anim/TwoHandSword_Attack1.TwoHandSword_Attack1" 1.0 "None"))
                (:1
                  (Variables|TwoHand|SetAttackCounter_TwoHand 2)
                  (Animation|PlayAnimMontage "/Game/_My/Weapon/Attack_Anim/TwoHandSword_Attack2.TwoHandSword_Attack2" 1.0 "None"))
                (:2
                  (Variables|TwoHand|SetAttackCounter_TwoHand 0)
                  (Animation|PlayAnimMontage "/Game/_My/Weapon/Attack_Anim/TwoHandSword_Attack3.TwoHandSword_Attack3" 1.0 "None"))))))))))

(fn ConstructionScript)

(fn EnableMouseCursor
  (bind _returnvalue (Game|GetPlayerController 0))
  (Input|SetInputModeGameandUI _returnvalue (Variables|Default|GetGameHUDReference) "DoNotLock" true)
  (Utilities|Casting|CastToHUD_InGame (HUD|GetHUD _returnvalue))
  (Variables|/Script/Engine.PlayerController|SetbShowMouseCursor _returnvalue true))

(fn DisalbeMouseCursor
  (bind _returnvalue (Game|GetPlayerController 0))
  (Input|SetInputModeGameOnly _returnvalue)
  (Utilities|Casting|CastToHUD_InGame (HUD|GetHUD _returnvalue))
  (Variables|/Script/Engine.PlayerController|SetbShowMouseCursor _returnvalue false))

(fn BlockAngleCheck
  (bind _returnvalue (Transformation|GetActorRotation))
  (bind _damage_causer (Variables|Default|GetDamage%20Causer))
  (bind _returnvalue_2 (Transformation|GetActorRotation _damage_causer))
  (bind _returnvalue_3 (- (.yaw _returnvalue) (.yaw _returnvalue_2)))
  (return (or (> _returnvalue_3 1.5e+02) (< _returnvalue_3 -1.5e+02))))